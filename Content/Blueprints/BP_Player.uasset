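; BP_Player is the player Blueprint, built on the Gameplay Ability System, and creates the HUD widget on BeginPlay.
; The Jump input activates the GA_Dodge ability, and the 1 key applies the GE_HealthRegen effect to itself.
; Tick prints current health against the base max health from the AttributeSet as an on-screen debug readout.
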(event `self.ReceiveBeginPlay`
  (bind _returnvalue (`|CreateWidget` "/GASCompanion/UI/WBP_HUD.WBP_HUD_C"))
  (`UserWidget.AddToViewport` _returnvalue 0))

(event `Key|One`
  (params (Key :type "Key Structure"))
  (bind _abilitysystemcomponent (`self.AbilitySystemComponent`))
  (:`Pressed`
    (`AbilitySystemComponent.BP_ApplyGameplayEffectToSelf` _abilitysystemcomponent "/GASCompanion/Abilities/StartingAttribute/GE_HealthRegen.GE_HealthRegen_C" 0.0 (`AbilitySystemComponent.MakeEffectContext` _abilitysystemcomponent))))

(event `InputAction|Jump`
  (params (Key :type "Key Structure"))
  (:`Pressed`
    (`AbilitySystemComponent.TryActivateAbilityByClass` (`self.AbilitySystemComponent`) "/GASCompanion/Abilities/StartingAbilities/GA_Dodge.GA_Dodge_C" true)))

(event `self.ReceiveTick`
  (params (DeltaSeconds :type "Float (single-precision)"))
  (bind _attributeset (`self.AttributeSet`))
  (`KismetSystemLibrary.PrintString` (`KismetTextLibrary.Conv_TextToString` (`|FormatText` "health: {health}/{maxHealth}" (`.CurrentValue` (break `GameplayAttributeData` (`GSCAttributeSet.Health` _attributeset))) (`.BaseValue` (break `GameplayAttributeData` (`GSCAttributeSet.MaxHealth` _attributeset))))) true true (struct :`G` 0.66 :`B` 1.0 :`A` 1.0) 0.0))

(fn `UserConstructionScript`)